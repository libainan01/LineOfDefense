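; BP_RTSAIController is the AI controller for RTS actors, linking their current state to a behavior tree.
; On BeginPlay it binds to the MonitorActorStates event and runs BT_RTSActorBehaviorTree.
; An event-style handler copies the AIBase state into the Blackboard, plus the data that state needs: move location, gather target or construction site.
; This updates the tree through events, with Tick left disabled.
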(event `self.ReceiveBeginPlay`
  (add `self.MonitorActorStates` (`|CreateDelegate` :!event `BP_RTSAIController_AutoGenFunc`))
  (`self.RunBehaviorTree` "/Game/Bluepirnt/Characters/AI/BehaviorTree/MianTree/BT_RTSActorBehaviorTree.BT_RTSActorBehaviorTree"))

(fn `BP_RTSAIController_AutoGenFunc`
  (params (NewActorType :type "CommandInfo Structure"))
  (bind _returnvalue (`RTSAIBase.GetActorStates` (`self.AIBase`)))
  (`BlackboardComponent.SetValueAsEnum` (`AIBlueprintHelperLibrary.GetBlackboard` null) "RTSActorState" _returnvalue)
  (switch `ERTSActorStates` _returnvalue
    (:`Moving`
      (`BlackboardComponent.SetValueAsVector` (`AIBlueprintHelperLibrary.GetBlackboard` null) "Location" (`.Location` (break `CommandInfo` (`local.NewActorType`)))))
    (:`Gathering`
      (`BlackboardComponent.SetValueAsObject` (`AIBlueprintHelperLibrary.GetBlackboard` null) "Material" (`KismetSystemLibrary.Conv_InterfaceToObject` (`.Target` (break `CommandInfo` (`local.NewActorType`))))))
    (:`Building`
      (`BlackboardComponent.SetValueAsObject` (`AIBlueprintHelperLibrary.GetBlackboard` null) "ConstructionSide" (`.ConstructionSide` (break `CommandInfo` (`local.NewActorType`)))))))

(fn `UserConstructionScript`)