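; BP_RTSWareHouse is an RTS warehouse that takes in gold and wood through the Gameplay Ability System.
; GetMaterials receives a Materials struct and applies GE_Gold and GE_Wood effect specs to the warehouse's own ability system component.
; Each resource amount is passed as the effect's Level rather than as a separate magnitude.
; The event graph holds only disabled stubs, and the construction script just calls its parent.
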(fn `GetMaterials`
  (params (Materials :type "Materials Structure"))
  (bind _returnvalue (`AbilitySystemBlueprintLibrary.GetAbilitySystemComponent` null))
  (bind _returnvalue_2 (`AbilitySystemBlueprintLibrary.GetAbilitySystemComponent` null))
  (`AbilitySystemComponent.BP_ApplyGameplayEffectSpecToSelf` _returnvalue_2 (`AbilitySystemComponent.MakeOutgoingSpec` _returnvalue_2 "/Game/Bluepirnt/Actors/GameEffect/GE_Gold.GE_Gold_C" (`KismetMathLibrary.Conv_IntToDouble` (`.Gold` (break `Materials` (`local.Materials`)))) (`AbilitySystemComponent.MakeEffectContext` _returnvalue_2)))
  (`AbilitySystemComponent.BP_ApplyGameplayEffectSpecToSelf` _returnvalue (`AbilitySystemComponent.MakeOutgoingSpec` _returnvalue "/Game/Bluepirnt/Actors/GameEffect/GE_Wood.GE_Wood_C" (`KismetMathLibrary.Conv_IntToDouble` (`.Wood` (break `Materials` (`local.Materials`)))) (`AbilitySystemComponent.MakeEffectContext` _returnvalue))))

(fn `UserConstructionScript`
  (`parent.UserConstructionScript`))